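; BP_Player is the player-controlled character, handling Enhanced Input setup and basic movement.
; On BeginPlay it adds the IMC_playerController mapping context to the local player's input subsystem.
; IA_Move stores side and forward input, then adds movement along the control rotation's right and forward vectors, and zeroes both values when input completes.
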(event Input|EnhancedActionEvents|EnhancedInputActionIA_Move
  (params (ActionValue :type Vector%202D%20Structure) (ElapsedSeconds :type Float%20%28double-precision%29) (TriggeredSeconds :type Float%20%28double-precision%29) (InputAction :type Input%20Action%20Object%20Reference :default "/Game/ARProject/Controller/InputAction/IA_Move.IA_Move"))
  (bind _returnvalue (Pawn|GetControlRotation :!class /Script/Engine.Pawn))
  ;[1 1 1] Move
  (:Triggered
    (Variables|Default|SetSideInput (.x ActionValue))
    (Variables|Default|SetForwardInput (.y ActionValue))
    (Pawn|Input|AddMovementInput (Math|Vector|GetRightVector _returnvalue) (Variables|Default|GetSideInput) false)
    (Pawn|Input|AddMovementInput (Math|Vector|GetForwardVector _returnvalue) (Variables|Default|GetForwardInput) false))
  (:Completed
    (Variables|Default|SetSideInput 0.0)
    (Variables|Default|SetForwardInput 0.0)))

(event EventBeginPlay
  ;[1 1 1] Input Mapping
  (bind _as플레이어_컨트롤러 (Utilities|Casting|CastToPlayerController (Pawn|GetController)))
  (Utilities|IsValid _as플레이어_컨트롤러
    (:Is%20Valid
      (Input|AddMappingContext (PlayerController|LocalPlayerSubsystems|GetEnhancedInputLocalPlayerSubsystem _as플레이어_컨트롤러) "/Game/ARProject/Controller/IMC_playerController.IMC_playerController" 0 "(bIgnoreAllPressedKeysUntilRelease=True,bForceImmediately=False)"))))

(fn ConstructionScript)